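; BP_witch is a witch character Blueprint that declares a set of spell events, from offensive casts like FireBall and Meteor to support skills like Recovery and ArcaneBarrier.
; Each spell event is a placeholder that only prints its own name, with no gameplay logic yet.
; BeginPlay, overlap, Tick and the construction script are empty, and nothing in this graph calls the spell events.
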(event Custom|FireBall
  (Development|PrintString "FireBall"))

(event Custom|WindBlast
  (Development|PrintString "WindBlast"))

(event Custom|IceSpear
  (Development|PrintString "IceSpear"))

(event Custom|Lightning
  (Development|PrintString "Lightning"))

(event Custom|Recovery
  (Development|PrintString "Recovery"))

(event Custom|ManaDrain
  (Development|PrintString "ManaDrain"))

(event Custom|Meteor
  (Development|PrintString "Meteor"))

(event Custom|ArcaneBarrier
  (Development|PrintString "ArcaneBarrier"))

(event Custom|HeartSanctuary
  (Development|PrintString "HeartSanctuary"))

(event Custom|ManaSurge
  (Development|PrintString "ManaSurge"))

(event EventBeginPlay)

(event Collision|EventActorBeginOverlap
  (params (OtherActor :type Actor%20Object%20Reference)))

(event EventTick
  (params (DeltaSeconds :type Float%20%28single-precision%29)))

(fn ConstructionScript)