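; Player controller that turns spell signals from a local HTTP server into spell casts on the player's witch.
; A looping timer polls the server's JSON spell field and forwards a recognized spell only when the value changes.
; ReceiveSpell sends a server cast request, where the player state validates and commits it.
; It also calls the matching spell on the controlled BP_witch without waiting for that validation.
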(event Custom|PollSpellSignal
  (bind _returnvalue (Class|HttpRequestProxyObject|CreateHttpRequestProxyObject "http://127.0.0.1:8000/signal" "GET"))
  (EventDispatchers|AssignOnRequestComplete _returnvalue (delegate Custom|OnRequestComplete_이벤트))
  (if (stale Custom|OnRequestComplete_이벤트 bSuccessful)
    (bind _outjsonobject (Class|JsonBlueprintFunctionLibrary|FromString (stale Custom|OnRequestComplete_이벤트 Response)))
    (bind _outvalue (|GetJsonField _outjsonobject "spell"))
    (if (Utilities|Enum|NotEqual(Enum) _outvalue (Variables|Default|GetLastSpell))
      (bind _output_get (Variables|Default|SetLastSpell _outvalue))
      (switch string _output_get
        (:fire_ball
          (CallFunction|ReceiveSpell "NewEnumerator0"))
        (:wind_blast
          (CallFunction|ReceiveSpell "NewEnumerator1"))
        (:ice_spear
          (CallFunction|ReceiveSpell "NewEnumerator2"))
        (:lightning
          (CallFunction|ReceiveSpell "NewEnumerator3"))
        (:recovery
          (CallFunction|ReceiveSpell "NewEnumerator4"))
        (:mana_drain
          (CallFunction|ReceiveSpell "NewEnumerator5"))
        (:meteor
          (CallFunction|ReceiveSpell "NewEnumerator6"))
        (:arcane_barrierNone
          (CallFunction|ReceiveSpell "NewEnumerator7"))
        (:heart_sanctuary
          (CallFunction|ReceiveSpell "NewEnumerator8"))
        (:mana_surge
          (CallFunction|ReceiveSpell "NewEnumerator9"))))
    (else
      (Development|PrintString "요청 실패"))))

(event Custom|OnRequestComplete_이벤트
  (params (Response :type String) (bSuccessful :type Boolean) (OutHeader :type Http%20Header%20Structure)))

(event Custom|ReceiveSpell
  (params (SpellID :type ESpellID%20Enum :default "NewEnumerator0"))
  (CallFunction|ServerRequestCast SpellID)
  (bind _asbp_witch (Utilities|Casting|CastToBP_witch (Pawn|GetControlledPawn)))
  (switch Utilities|FlowControl|Switch|SwitchonESpellID SpellID
    (:NewEnumerator0
      (Default|FireBall _asbp_witch))
    (:NewEnumerator1
      (Default|WindBlast _asbp_witch))
    (:NewEnumerator2
      (Default|IceSpear _asbp_witch))
    (:NewEnumerator3
      (Default|Lightning _asbp_witch))
    (:NewEnumerator4
      (Default|Recovery _asbp_witch))
    (:NewEnumerator5
      (Default|ManaDrain _asbp_witch))
    (:NewEnumerator6
      (Default|Meteor _asbp_witch))
    (:NewEnumerator7
      (Default|ArcaneBarrier _asbp_witch))
    (:NewEnumerator8
      (Default|HeartSanctuary _asbp_witch))
    (:NewEnumerator9
      (Default|ManaSurge _asbp_witch))))

(event Custom|Server_RequestCast
  (params (SpellID :type ESpellID%20Enum :default "NewEnumerator0"))
  (bind _asbp_spell_cast_player_state (Utilities|Casting|CastToBP_SpellCastPlayerState (Variables|GetPlayerState)))
  (bind _cancast (Default|CanCastSpell _asbp_spell_cast_player_state SpellID))
  (if _cancast
    (Default|CommitCast _asbp_spell_cast_player_state SpellID)
    (Development|PrintString (Utilities|String|ToString(Integer) (Variables|/Game/blueprints/BP_SpellCastPlayerState.BP_SpellCastPlayerState_C|GetMana _asbp_spell_cast_player_state)))))

(event EventBeginPlay
  (Development|PrintString "서버테스트")
  (Utilities|Time|SetTimerbyEvent (delegate Custom|PollSpellSignal) 0.1 true))

(event EventTick
  (params (DeltaSeconds :type Float%20%28single-precision%29)))

(fn ConstructionScript)