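; Witch actor Blueprint that casts ten named spells, each exposed as a custom event that prints its name and calls a matching Play function.
; Most Play functions spawn that spell's Blueprint at the witch's transform, with Fireball raised above and Wind Blast offset forward.
; Lightning instead spawns a bolt on every actor tagged "enemy".
; Ice Spear, Mana Drain and Meteor are empty stubs, and nothing here triggers the events.
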(event Custom|FireBall
  (Development|PrintString "FireBall")
  (CallFunction|PlayFireBall))

(event Custom|WindBlast
  (Development|PrintString "WindBlast")
  (CallFunction|PlayWindBlast))

(event Custom|IceSpear
  (Development|PrintString "IceSpear")
  (CallFunction|PlayIceSpear))

(event Custom|Lightning
  (Development|PrintString "Lightning")
  (CallFunction|PlayLightning))

(event Custom|Recovery
  (Development|PrintString "Recovery")
  (CallFunction|PlayRecovery))

(event Custom|ManaDrain
  (Development|PrintString "ManaDrain")
  (CallFunction|PlayManaDrain))

(event Custom|Meteor
  (Development|PrintString "Meteor")
  (CallFunction|PlayMeteor))

(event Custom|ArcaneBarrier
  (Development|PrintString "ArcaneBarrier")
  (CallFunction|PlayArcaneBarrier))

(event Custom|HeartSanctuary
  (Development|PrintString "HeartSanctuary")
  (CallFunction|PlayHeartSanctuary))

(event Custom|ManaSurge
  (Development|PrintString "ManaSurge")
  (CallFunction|PlayManaSurge))

(event EventBeginPlay)

(event Collision|EventActorBeginOverlap
  (params (OtherActor :type Actor%20Object%20Reference)))

(event EventTick
  (params (DeltaSeconds :type Float%20%28single-precision%29)))

(fn ConstructionScript)

(fn PlayFireBall
  (bind _returnvalue (Transformation|GetActorTransform))
  (Game|SpawnActorfromClass "/Game/blueprints/spells/FireBall/BP_FireBall.BP_FireBall_C" (Math|Transform|MakeTransform (Math|Vector|MakeVector (.x (.location _returnvalue)) (.y (.location _returnvalue)) (+ (.z (.location _returnvalue)) 1e+02)) (.rotation _returnvalue) (.scale _returnvalue)) "Undefined" "MultiplyWithRoot" 0 0))

(fn PlayWindBlast
  (bind _returnvalue (Transformation|GetActorTransform))
  (Game|SpawnActorfromClass "/Game/blueprints/spells/WindBlast/BP_WindBlast.BP_WindBlast_C" (Math|Transform|MakeTransform (+ (* (Transformation|GetActorForwardVector) "50.000000,50.000000,50.000000") (.location _returnvalue)) (.rotation _returnvalue) (.scale _returnvalue)) "Undefined" "MultiplyWithRoot" 0 0))

(fn PlayIceSpear)

(fn PlayLightning
  (bind _outactors (Actor|GetAllActorswithTag "enemy"))
  (for _array_element _outactors
    (Game|SpawnActorfromClass "/Game/blueprints/spells/Lightning/BP_Lightning.BP_Lightning_C" (Math|Transform|MakeTransform (.location (Transformation|GetActorTransform _array_element)) "0, 0, 0" "1.000000,1.000000,1.000000") "Undefined" "MultiplyWithRoot" 0 0)))

(fn PlayRecovery
  (bind _returnvalue (Transformation|GetActorTransform))
  (Game|SpawnActorfromClass "/Game/blueprints/spells/Recovery/BP_Recovery.BP_Recovery_C" (Math|Transform|MakeTransform (.location _returnvalue) (.rotation _returnvalue) (.scale _returnvalue)) "Undefined" "MultiplyWithRoot" 0 0))

(fn PlayManaDrain)

(fn PlayMeteor)

(fn PlayArcaneBarrier
  (bind _returnvalue (Transformation|GetActorTransform))
  (Game|SpawnActorfromClass "/Game/blueprints/spells/ArcaneBarrier/BP_ArcaneBarrier.BP_ArcaneBarrier_C" (Math|Transform|MakeTransform (.location _returnvalue) (.rotation _returnvalue) (.scale _returnvalue)) "Undefined" "MultiplyWithRoot" 0 0))

(fn PlayHeartSanctuary
  (bind _returnvalue (Transformation|GetActorTransform))
  (Game|SpawnActorfromClass "/Game/blueprints/spells/HeartSanctuary/BP_HeartSanctuary.BP_HeartSanctuary_C" (Math|Transform|MakeTransform (.location _returnvalue) (.rotation _returnvalue) (.scale _returnvalue)) "Undefined" "MultiplyWithRoot" 0 0))

(fn PlayManaSurge
  (bind _returnvalue (Transformation|GetActorTransform))
  (Game|SpawnActorfromClass "/Game/blueprints/spells/ManaSurge/BP_ManaSurge.BP_ManaSurge_C" (Math|Transform|MakeTransform (.location _returnvalue) (.rotation _returnvalue) (.scale _returnvalue)) "Undefined" "MultiplyWithRoot" 0 0))