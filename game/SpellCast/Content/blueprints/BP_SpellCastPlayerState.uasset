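; Player State for a spell-casting game, holding a player's mana and spell cycle alongside HP and Barrier, with empty RepNotify handlers for each.
; A server-only looping timer regenerates mana up to MaxMana.
; Only the first three spells in the cycle are castable, if mana covers the DT_SpellData cost.
; CommitCast deducts that cost, debug-prints it and moves the spell to the back of the cycle, like a card rotation.
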(event EventBeginPlay
  (if (Ability|HasAuthority)
    (Utilities|Time|SetTimerbyFunctionName 0 "RegenerateMana" 2.0 true 2.0)))

(event EventTick
  (params (DeltaSeconds :type Float%20%28single-precision%29)))

(fn ConstructionScript)

(fn OnRepHP)

(fn OnRepMana)

(fn OnRepSpellCycle)

(fn OnRepBarrier)

(fn GetSpellCost
  (params (SpellID :type ESpellID%20Enum :default "NewEnumerator0"))
  (bind _returnvalue (Utilities|GetDataTableRow "/Game/blueprints/DT_SpellData.DT_SpellData" (Utilities|String|StringToName (Utilities|String|EnumtoString SpellID)))
    (:then
      (return (.cost _returnvalue)))
    (:RowNotFound
      (return 999))))

(fn CanCastSpell
  (params (Spell :type ESpellID%20Enum :default "NewEnumerator0"))
  (bind _spellcycle (Variables|Default|GetSpellCycle))
  (if (>= (Utilities|Array|Length _spellcycle) 3)
    (bind _spellcost (CallFunction|GetSpellCost Spell))
    (return (and (Math|Boolean|ORBoolean (Utilities|Enum|Equal(Enum) Spell (Utilities|Array|Get(acopy) _spellcycle)) (Utilities|Enum|Equal(Enum) Spell (Utilities|Array|Get(acopy) _spellcycle 1)) (Utilities|Enum|Equal(Enum) Spell (Utilities|Array|Get(acopy) _spellcycle 2))) (>= (Variables|Default|GetMana) _spellcost)))
    (else
      (return false))))

(fn CommitCast
  (params (SpellID :type ESpellID%20Enum :default "NewEnumerator0"))
  (bind _spellcycle (Variables|Default|GetSpellCycle))
  (bind _spellcost (CallFunction|GetSpellCost SpellID))
  (Variables|Default|SetMana (- (Variables|Default|GetMana) _spellcost))
  (Development|PrintString (Utilities|String|ToString(Integer) _spellcost))
  (Utilities|Array|RemoveItem _spellcycle SpellID)
  (Utilities|Array|Add _spellcycle SpellID))

(fn RegenerateMana
  (if (Ability|HasAuthority)
    (if (< (Variables|Default|GetMana) (Variables|Default|GetMaxMana))
      (Math|Integer|IncrementInt (Variables|Default|GetMana)))))

(fn GetSpellName
  (params (SpellID :type ESpellID%20Enum :default "NewEnumerator0"))
  (bind _returnvalue (Utilities|GetDataTableRow "/Game/blueprints/DT_SpellData.DT_SpellData" (Utilities|String|StringToName (Utilities|String|EnumtoString SpellID)))
    (:then
      (return (.displayname _returnvalue)))
    (:RowNotFound
      (return "None"))))