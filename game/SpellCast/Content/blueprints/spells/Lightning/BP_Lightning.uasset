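; BP_Lightning is a short-lived lightning spell actor that plays a timed visual sequence and then removes itself.
; On BeginPlay it hides Lightning2 and Lightning3, then uses short delays to hand visibility from Lightning1 to Lightning3 to Lightning2.
; The actor is destroyed immediately after Lightning2 is shown, with no delay for that last stage.
; Overlap, Tick and the construction script are empty.
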(event EventBeginPlay
  (Rendering|SetVisibility (Variables|Default|Getlightning3) false false)
  (Rendering|SetVisibility (Variables|Default|Getlightning2) false false)
  (Utilities|FlowControl|Delay 0.5)
  (Rendering|SetVisibility (Variables|Default|Getlightning1) false false)
  (Rendering|SetVisibility (Variables|Default|Getlightning3) true false)
  (Utilities|FlowControl|Delay 0.5)
  (Rendering|SetVisibility (Variables|Default|Getlightning3) false false)
  (Rendering|SetVisibility (Variables|Default|Getlightning2) true false)
  (Actor|DestroyActor))

(event Collision|EventActorBeginOverlap
  (params (OtherActor :type Actor%20Object%20Reference)))

(event EventTick
  (params (DeltaSeconds :type Float%20%28single-precision%29)))

(fn ConstructionScript)