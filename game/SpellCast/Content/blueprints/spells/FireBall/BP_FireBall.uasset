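; BP_FireBall is a fireball spell projectile launched toward the player controller's target pawn.
; On BeginPlay it casts the first player controller to BP_playercontroller and sets ProjectileMovement velocity from the offset to TargetPawn.
; Dividing that offset by a fixed flight time and adding upward speed suggests a gravity-compensated arc, with no homing afterward.
; Overlap and Tick are empty, so this graph has no hit logic.
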(event EventBeginPlay
  (bind _asbp_playercontroller (Utilities|Casting|CastToBP_playercontroller (Game|GetPlayerController 0)))
  (Variables|/Script/Engine.MovementComponent|SetVelocity (Variables|Default|GetProjectileMovement) (Math|Vector|MakeVector (/ (.x (- (Transformation|GetActorLocation (Variables|/Game/blueprints/BP_playercontroller.BP_playercontroller_C|GetTargetPawn _asbp_playercontroller)) (.location (Transformation|GetActorTransform)))) 3.0) (/ (.y (- (Transformation|GetActorLocation (Variables|/Game/blueprints/BP_playercontroller.BP_playercontroller_C|GetTargetPawn _asbp_playercontroller)) (.location (Transformation|GetActorTransform)))) 3.0) (+ (/ (.z (- (Transformation|GetActorLocation (Variables|/Game/blueprints/BP_playercontroller.BP_playercontroller_C|GetTargetPawn _asbp_playercontroller)) (.location (Transformation|GetActorTransform)))) 3.0) 147.0))))

(event Collision|EventActorBeginOverlap
  (params (OtherActor :type Actor%20Object%20Reference)))

(event EventTick
  (params (DeltaSeconds :type Float%20%28single-precision%29)))

(fn ConstructionScript)